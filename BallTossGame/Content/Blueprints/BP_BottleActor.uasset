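; Knockable bottle target that detects when it has been knocked over and can return to its starting pose.
; While simulating physics, Tick checks for a height drop or tilt past a threshold, then fires OnKO once and swaps the material.
; ReturnToStart disables physics and collision, eases the actor back on a timeline scaled by TimeToReturn, then restores material and physics and re-arms detection.
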(event `self.ReceiveBeginPlay`
  (bind _staticmesh (`self.StaticMesh`))
  (set `self.StartingRotation` (`SceneComponent.K2_GetComponentRotation` _staticmesh))
  (set `self.StartingLocation` (`SceneComponent.K2_GetComponentLocation` _staticmesh)))

(event `self.ReceiveTick`
  (params (DeltaSeconds :type "Float (single-precision)"))
  (bind (_startinglocation_x _startinglocation_y _startinglocation_z) (`KismetMathLibrary.BreakVector` (`self.StartingLocation`)))
  (bind _staticmesh (`self.StaticMesh`))
  (bind (_returnvalue_x _returnvalue_y _returnvalue_z) (`KismetMathLibrary.BreakVector` (`SceneComponent.K2_GetComponentLocation` _staticmesh)))
  (bind (_returnvalue_roll _returnvalue_pitch) (`KismetMathLibrary.BreakRotator` (`KismetMathLibrary.NormalizedDeltaRotator` (`SceneComponent.K2_GetComponentRotation` _staticmesh) (`self.StartingRotation`))))
  ;[1 1 1] Checks each tick if bottle has been knocked over
  (if (`SceneComponent.IsAnySimulatingPhysics` (`self.StaticMesh`))
    (bind _output_get (set `self.Knocked Over?` (or (> (- _startinglocation_z _returnvalue_z) 30.0) (> (`KismetMathLibrary.VSize2D` (`KismetMathLibrary.MakeVector2D` _returnvalue_roll _returnvalue_pitch)) 45.0))))
    (if _output_get
      (`/Engine/EditorBlueprintResources/StandardMacros.DoOnce` false :!label _label
        (:`Completed`
          (`self.OnKO`)
          (`PrimitiveComponent.SetMaterial` (`self.StaticMesh`) 0 "/Game/VRTemplate/Materials/MI_Projectile.MI_Projectile"))))))

(event `ReturnToStart`
  (bind _staticmesh (`self.StaticMesh`))
  ;[1 1 1] Resets Bottle to starting transform and status
  (`PrimitiveComponent.SetSimulatePhysics` _staticmesh false)
  (`PrimitiveComponent.SetCollisionEnabled` _staticmesh "NoCollision")
  (`TimelineComponent.SetPlayRate` (`self.CurveLerp`) (/ 1.0 (`self.TimeToReturn`)))
  (bind (_direction _progress) (`Timeline|CurveLerp` :!via `PlayFromStart`)
    (:`Update`
      (`self.K2_SetActorLocation` (`KismetMathLibrary.VLerp` (`self.K2_GetActorLocation`) (`self.StartingLocation`) _progress))
      (`self.K2_SetActorRotation` (`KismetMathLibrary.RLerp` (`self.K2_GetActorRotation`) (`self.StartingRotation`) _progress)))
    (:`Finished`
      (`PrimitiveComponent.SetCollisionEnabled` _staticmesh "QueryAndPhysics")
      (`PrimitiveComponent.SetMaterial` _staticmesh 0 "/Game/Megascans/Surfaces/Scratched_Anodized_Aluminum_sgsocjfc/MI_Scratched_Anodized_Aluminum_sgsocjfc_1K.MI_Scratched_Anodized_Aluminum_sgsocjfc_1K")
      (set `self.Knocked Over?` false)
      (`PrimitiveComponent.SetSimulatePhysics` _staticmesh true)
      (goto _label :!via `Reset`))))

(fn `UserConstructionScript`)