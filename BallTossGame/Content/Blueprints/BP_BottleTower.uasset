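; BP_BottleTower manages a set of knock-over bottles and resets them once all have fallen.
; On BeginPlay it binds to each bottle's OnKO event and counts every knockdown.
; When the count reaches the number of bottles, it waits briefly, then clears the counter and tells each bottle to return to its start.
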(event `self.ReceiveBeginPlay`
  (for _array_element (`self.Bottles`)
    (add `/Game/Blueprints/BP_BottleActor.OnKO` _array_element (delegate `BottleKnockedOver`))))

(event `BottleKnockedOver`
  (bind _result (`/Engine/EditorBlueprintResources/StandardMacros.IncrementInt` (`self.NumKnockedOver`))
    (:`  `
      (if (>= _result (`KismetArrayLibrary.Array_Length` (`self.Bottles`)))
        (`KismetSystemLibrary.Delay` 5.0)
        (`self.ResetAll`)))))

(event `ResetAll`
  (set `self.NumKnockedOver` 0)
  (for _array_element (`self.Bottles`)
    (`/Game/Blueprints/BP_BottleActor.ReturnToStart` _array_element)))

(fn `UserConstructionScript`)